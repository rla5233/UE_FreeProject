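; Player character for CombatRobot that runs automatically along a spline, reversing direction on right click.
; Left click deprojects the mouse, traces toward it in the X/Z plane, then teleports onto a hit air enemy or to the nearest spline point.
; Grabbing pauses spline movement; a second click or two-second timeout destroys the enemy and snaps back to the spline, aimed at the cursor or along the grab direction.
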(event `self.ReceiveTick`
  (params (DeltaSeconds :type "Float (single-precision)"))
  (bind _returnvalue (`self.K2_GetActorLocation`))
  (bind _distancealongspline (`self.DistanceAlongSpline`))
  (bind _splineref (`self.SplineRef`))
  (bind _spline (`/Game/BluePrint/CombatRobot/GameSystem/SplineSystem/BP_CombatRobot_SplinePath.Spline` (`self.SplineRef`)))
  (bind _returnvalue_2 (`SplineComponent.GetSplineLength` (`/Game/BluePrint/CombatRobot/GameSystem/SplineSystem/BP_CombatRobot_SplinePath.Spline` (`self.SplineRef`))))
  ; 캐릭터 이동
  (if (`self.bGrapEnemy`)
    ; 공중적 붙잡기
    (bind _output_get (set `self.GrapTime` (+ (`self.GrapTime`) DeltaSeconds)))
    (if (>= _output_get 2.0)
      (`self.K2_DestroyActor` (`self.GrapEnemy`))
      (set `self.bGrapEnemy` false)
      (set `self.GrapTime` 0.0)
      (bind _outhit (`KismetSystemLibrary.LineTraceSingle` :`Start` _returnvalue :`End` (+ _returnvalue (* (`self.LineTraceDir`) 1000.0)) :`TraceChannel` "TraceTypeQuery1" :`DrawDebugType` "ForDuration"))
      (bind _returnvalue_3 (`SplineComponent.FindInputKeyClosestToWorldLocation` _spline (`.Location` (`GameplayStatics.BreakHitResult` _outhit))))
      (`self.K2_SetActorLocation` (`SplineComponent.GetLocationAtDistanceAlongSpline` _spline _returnvalue_3 "World"))
      (set `self.DistanceAlongSpline` (`SplineComponent.GetDistanceAlongSplineAtSplineInputKey` _spline _returnvalue_3)))
    (else
      (`/Engine/EditorBlueprintResources/StandardMacros.IsValid` (`self.SplineRef`)
        (:`Is Valid`
          (bind _output_get_2 (set `self.DistanceAlongSpline` (+ (`self.DistanceAlongSpline`) (* DeltaSeconds (`self.MoveSpeed`)))))
          (if (>= _output_get_2 0.0)
            (set `self.DistanceAlongSpline` (mod (`self.DistanceAlongSpline`) _returnvalue_2))
            (else
              (set `self.DistanceAlongSpline` (- _returnvalue_2 (`self.DistanceAlongSpline`)))))
          (`self.K2_SetActorTransform` (`KismetMathLibrary.MakeTransform` (`SplineComponent.GetLocationAtDistanceAlongSpline` (`/Game/BluePrint/CombatRobot/GameSystem/SplineSystem/BP_CombatRobot_SplinePath.Spline` _splineref) _distancealongspline "World") (`SplineComponent.GetRotationAtDistanceAlongSpline` (`/Game/BluePrint/CombatRobot/GameSystem/SplineSystem/BP_CombatRobot_SplinePath.Spline` _splineref) _distancealongspline "Local"))))))))

(event `Key|RightMouseButton`
  (params (Key :type "Key Structure"))
  ; RButtion Click
  (:`Pressed`
    (set `self.MoveSpeed` (* (`self.MoveSpeed`) -1.0))))

(event `Key|LeftMouseButton`
  (params (Key :type "Key Structure"))
  (bind _returnvalue (`self.K2_GetActorLocation`))
  (bind _returnvalue_2 (`self.K2_GetActorLocation`))
  (bind (_worldlocation _worlddirection) (`PlayerController.DeprojectMousePositionToWorld` (`GameplayStatics.GetPlayerController` 0)))
  (bind (_worldlocation_2 _worlddirection_2) (`PlayerController.DeprojectMousePositionToWorld` (`GameplayStatics.GetPlayerController` 0)))
  (bind _spline (`/Game/BluePrint/CombatRobot/GameSystem/SplineSystem/BP_CombatRobot_SplinePath.Spline` (`self.SplineRef`)))
  (bind _spline_2 (`/Game/BluePrint/CombatRobot/GameSystem/SplineSystem/BP_CombatRobot_SplinePath.Spline` (`self.SplineRef`)))
  ; LButtion Click (잡기 상태 아닐 시)
  (:`Pressed`
    (if (`self.bGrapEnemy`)
      ; LButtion Click (잡기 상태 일시)
      (bind _outhit (`KismetSystemLibrary.LineTraceSingle` _worldlocation (+ _worldlocation (* _worlddirection 5000.0)) "TraceTypeQuery1"))
      (bind (_returnvalue_x _returnvalue_y _returnvalue_z) (`KismetMathLibrary.BreakVector` (- (`.Location` (`GameplayStatics.BreakHitResult` _outhit)) _returnvalue)))
      (bind _outhit_2 (`KismetSystemLibrary.LineTraceSingle` :`Start` _returnvalue :`End` (+ _returnvalue (* (`KismetMathLibrary.Normal` (`KismetMathLibrary.MakeVector` _returnvalue_x 0.0 _returnvalue_z)) 5000.0)) :`TraceChannel` "TraceTypeQuery1" :`DrawDebugType` "ForDuration"))
      (`self.K2_DestroyActor` (`self.GrapEnemy`))
      (set `self.bGrapEnemy` false)
      (set `self.GrapTime` 0.0)
      (bind _returnvalue_3 (`SplineComponent.FindInputKeyClosestToWorldLocation` _spline (`.Location` (`GameplayStatics.BreakHitResult` _outhit_2))))
      (`self.K2_SetActorLocation` (`SplineComponent.GetLocationAtDistanceAlongSpline` _spline _returnvalue_3 "World"))
      (set `self.DistanceAlongSpline` (`SplineComponent.GetDistanceAlongSplineAtSplineInputKey` _spline _returnvalue_3))
      (else
        (bind _outhit_3 (`KismetSystemLibrary.LineTraceSingle` _worldlocation_2 (+ _worldlocation_2 (* _worlddirection_2 5000.0)) "TraceTypeQuery1"))
        (bind (_returnvalue_x_2 _returnvalue_y_2 _returnvalue_z_2) (`KismetMathLibrary.BreakVector` (- (`.Location` (`GameplayStatics.BreakHitResult` _outhit_3)) _returnvalue_2)))
        (bind _outhit_4 (`KismetSystemLibrary.LineTraceSingle` :`Start` _returnvalue_2 :`End` (+ _returnvalue_2 (* (`KismetMathLibrary.Normal` (`KismetMathLibrary.MakeVector` _returnvalue_x_2 0.0 _returnvalue_z_2)) 5000.0)) :`TraceChannel` "TraceTypeQuery1" :`DrawDebugType` "ForOneFrame"))
        (bind _asbp_air_enemy (cast `/Game/BluePrint/CombatRobot/GameSystem/EnemySystem/BP_AirEnemy` (`.HitActor` (`GameplayStatics.BreakHitResult` _outhit_4)))
          (:`then`
            (bind _output_get (set `self.GrapEnemy` _asbp_air_enemy))
            (`PrimitiveComponent.SetCollisionEnabled` (`/Game/BluePrint/CombatRobot/GameSystem/EnemySystem/BP_Enemy.Body` _output_get) "NoCollision")
            (set `self.bGrapEnemy` true)
            (bind _returnvalue_4 (`self.K2_GetActorLocation` _output_get))
            (bind (_returnvalue_x_3 _returnvalue_y_3 _returnvalue_z_3) (`KismetMathLibrary.BreakVector` (- _returnvalue_4 (`self.K2_GetActorLocation`))))
            (set `self.LineTraceDir` (`KismetMathLibrary.Normal` (`KismetMathLibrary.MakeVector` _returnvalue_x_3 0.0 _returnvalue_z_3)))
            (`self.K2_SetActorLocation` _returnvalue_4))
          (:`CastFailed`
            (bind _returnvalue_5 (`SplineComponent.FindInputKeyClosestToWorldLocation` _spline_2 (`.Location` (`GameplayStatics.BreakHitResult` _outhit_4))))
            (`self.K2_SetActorLocation` (`SplineComponent.GetLocationAtDistanceAlongSpline` _spline_2 _returnvalue_5 "World"))
            (set `self.DistanceAlongSpline` (`SplineComponent.GetDistanceAlongSplineAtSplineInputKey` _spline_2 _returnvalue_5))))))))

(fn `UserConstructionScript`)